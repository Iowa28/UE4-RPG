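; Enemy character Blueprint that carries a lock-on target icon for the targeting system.
; On BeginPlay it casts the TargetLockIcon component's widget to WBP_TargetLock, caches it and hides it.
; The UpdateTargetIcon event takes a Show flag and calls ShowTarget or HideTarget on the cached widget.
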(event EventBeginPlay
  (bind _aswbp_target_lock (Utilities|Casting|CastToWBP_TargetLock (UserInterface|GetUserWidgetObject (Variables|Default|GetTargetLockIcon))))
  (bind _output_get (Variables|Default|SetTargetLock _aswbp_target_lock))
  (Default|HideTarget _output_get))

(event EventUpdateTargetIcon
  (params (bShow :type Boolean))
  (if bShow
    (Default|ShowTarget (Variables|Default|GetTargetLock))
    (else
      (Default|HideTarget (Variables|Default|GetTargetLock)))))

(fn ConstructionScript)